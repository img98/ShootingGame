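; Server-authoritative spawner that places a random actor from its Items list at its own transform on BeginPlay.
; A randomly timed ChangeItem call swaps a still-valid item for a new random pick, restarting the cycle through SpawnItem.
; An OnDestroyed binding schedules a delayed respawn when the item is destroyed, and is unbound before swaps so they do not trigger it.
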(event EventBeginPlay
  (CallFunction|SpawnItem))

(fn ConstructionScript)

(fn SpawnItem
  (Networking|SwitchHasAuthority
    (:Authority
      (Utilities|FlowControl|Sequence
        (:then_0
          (CallFunction|CreateItem))
        (:then_1
          (Utilities|Time|SetTimerbyFunctionName 0 "ChangeItem" (Math|Random|RandomFloatinRange 5.0 1e+01)))))))

(fn EventItemDestroy
  (params (DestroyedActor :type Actor%20Object%20Reference))
  (Utilities|Time|SetTimerbyFunctionName 0 "SpawnItem" 5.0))

(fn ChangeItem
  (bind _spawneditem (Variables|Default|GetSpawnedItem)
    (:then
      (bind _output_get (LocalVariables|SetOldItem _spawneditem))
      (Game|UnbindEventfromOnDestroyed _output_get (EventDispatchers|CreateEvent :!event EventItemDestroy))
      (CallFunction|SpawnItem)
      (Actor|DestroyActor (LocalVariables|GetOldItem)))
    (:else)))

(fn CreateItem
  (bind _items (Variables|Default|GetItems))
  (if (Utilities|Array|IsNotEmpty _items)
    (bind _returnvalue (Game|SpawnActorfromClass (.OutItem (Utilities|Array|Random _items)) (Transformation|GetActorTransform) "Undefined" "MultiplyWithRoot" 0 0))
    (bind _output_get (Variables|Default|SetSpawnedItem _returnvalue))
    (Game|BindEventtoOnDestroyed _output_get (EventDispatchers|CreateEvent :!event EventItemDestroy))))