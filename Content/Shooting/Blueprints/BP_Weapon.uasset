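; Networked, data-driven weapon that characters grab, drop, fire and reload, with mesh, damage, ammo, fire rate and montages taken from WeaponData.
; Fire plays muzzle effects, and only the owning player requests the server hit check, a camera-aimed line trace that damages shooting characters.
; Reload spends a magazine from the PlayerState to refill ammo.
; Ammo's OnRep fires a dispatcher that grab and drop bind to or unbind from the local HUD.
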(event Custom|ReqShoot
  (params (StartVector :type Vector) (EndVector :type Vector))
  (CallFunction|UseAmmo)
  (bind _outhit (Collision|LineTraceForObjects StartVector EndVector (Utilities|Array|MakeArray "ObjectTypeQuery1" "ObjectTypeQuery2" "ObjectTypeQuery3" "ObjectTypeQuery4" "ObjectTypeQuery5" "ObjectTypeQuery6") false 0 "ForOneFrame"))
  (bind _asbp_shooting_character (Utilities|Casting|CastToBP_ShootingCharacter (.HitActor (Collision|BreakHitResult _outhit))))
  (Game|Damage|ApplyDamage _asbp_shooting_character (.Damage (Utilities|Struct|BreakST_WeaponData (Variables|Default|GetWeaponData))) (Pawn|GetController (Variables|Default|GetCharacter)) self))

(event Custom|ReqReload
  ;[1 1 1] 플레이어 Mag감소
  (bind _asbp_shooting_player_state (Utilities|Casting|CastToBP_ShootingPlayerState (Variables|/Script/Engine.Pawn|GetPlayerState (Variables|Default|GetCharacter))))
  (bind _isuse (Default|UseMag _asbp_shooting_player_state))
  (if _isuse
    ;[1 1 1] 무기 Ammo증가
    (CallFunction|ChangeMag)))

(event EventBeginPlay
  (CallFunction|InitWeapon))

(fn ConstructionScript)

(fn CalcStartForwardVector
  (params (MuzzleLoc :type Vector))
  (bind _returnvalue (Game|GetPlayerCameraManager 0))
  (bind _returnvalue_2 (Transformation|GetActorForwardVector _returnvalue))
  (bind _returnvalue_3 (Transformation|GetActorLocation _returnvalue))
  (return (+ _returnvalue_3 (* _returnvalue_2 (Math|Vector|Distance(Vector) MuzzleLoc _returnvalue_3))) (+ _returnvalue_3 (* _returnvalue_2 5e+03))))

(fn OnRepAmmo
  (Default|CallEventDispatcherUpdateAmmo (Variables|Default|GetAmmo)))

(fn UseAmmo
  (Variables|Default|SetAmmo (- (Variables|Default|GetAmmo) 1)))

(fn BindAmmo
  (bind _returnvalue (Game|GetPlayerController 0))
  (if (== (Variables|Default|GetCharacter) (Pawn|GetControlledPawn _returnvalue))
    (bind _asbp_shooting_hud (Utilities|Casting|CastToBP_ShootingHud (HUD|GetHUD _returnvalue)))
    (Default|EventMyAmmo _asbp_shooting_hud (Variables|Default|GetAmmo))
    (EventDispatchers|BindEventtoEventDispatcherUpdateAmmo (EventDispatchers|CreateEvent _asbp_shooting_hud :!event EventMyAmmo))))

(fn UnBindAmmo
  (bind _returnvalue (Game|GetPlayerController 0))
  (if (== (Variables|Default|GetCharacter) (Pawn|GetControlledPawn _returnvalue))
    (bind _asbp_shooting_hud (Utilities|Casting|CastToBP_ShootingHud (HUD|GetHUD _returnvalue)))
    (EventDispatchers|UnbindEventfromEventDispatcherUpdateAmmo (EventDispatchers|CreateEvent _asbp_shooting_hud :!event EventMyAmmo))
    (Default|EventMyAmmo _asbp_shooting_hud)))

(fn ChangeMag
  (Variables|Default|SetAmmo (.MaxAmmo (Utilities|Struct|BreakST_WeaponData (Variables|Default|GetWeaponData)))))

(fn IsCanChangeMag
  (bind _character (Variables|Default|GetCharacter)
    (:then
      (bind _asbp_shooting_player_state (Utilities|Casting|CastToBP_ShootingPlayerState (Variables|/Script/Engine.Pawn|GetPlayerState _character))
        (:then
          (if (Default|IsCanUseMag _asbp_shooting_player_state)
            (return true)
            (else
              (return false))))
        (:CastFailed
          (return false))))
    (:else
      (return false))))

(fn InitWeapon
  (Components|StaticMesh|SetStaticMesh (Variables|Default|GetStaticMesh) (.StaticMesh (Utilities|Struct|BreakST_WeaponData (Variables|Default|GetWeaponData))))
  (CallFunction|ChangeMag))

(fn GetFireDelaybyRPM
  (return (/ 1.0 (/ (.RPM (Utilities|Struct|BreakST_WeaponData (Variables|Default|GetWeaponData))) 60))))

(fn EventDrop
  (params (Character :type Character%20Object%20Reference))
  (bind _staticmesh (Variables|Default|GetStaticMesh))
  (CallFunction|UnBindAmmo)
  (Collision|SetCollisionEnabled _staticmesh "QueryAndPhysics")
  (Physics|SetSimulatePhysics _staticmesh true)
  (Transformation|DetachFromComponent _staticmesh "KeepWorld" "KeepWorld" "KeepWorld" true)
  (Variables|Default|SetCharacter 0)
  (return true))

(fn EventFire
  (bind _staticmesh (Variables|Default|GetStaticMesh))
  (bind _returnvalue (Transformation|GetSocketTransform _staticmesh "Muzzle" "RTS_World"))
  (bind (_startvec _endvec) (CallFunction|CalcStartForwardVector (.location _returnvalue)))
  (bind _iscanfire (CallFunction|IsCanFire))
  (if _iscanfire
    (Effects|SpawnEmitteratLocation "/Game/StarterContent/Particles/P_Explosion.P_Explosion" (.location _returnvalue) (.rotation _returnvalue) "0.100000,0.100000,0.100000")
    (Audio|SpawnSoundatLocation "/Game/StarterContent/Audio/Explosion_Cue.Explosion_Cue" (.location _returnvalue) "0, 0, 0" 1.0 1.0 0.0 0 0)
    (Utilities|IsOwner?
      (:True
        (CallFunction|ReqShoot _startvec _endvec)
        (return true)))))

(fn EventGrab
  (params (Character :type Character%20Object%20Reference))
  (bind _staticmesh (Variables|Default|GetStaticMesh))
  (bind _output_get (Variables|Default|SetCharacter Character))
  (Physics|SetSimulatePhysics _staticmesh false)
  (Collision|SetCollisionEnabled _staticmesh "NoCollision")
  (Transformation|AttachComponentToComponent _staticmesh (Variables|/Script/Engine.Character|GetMesh _output_get) "weapon" "SnapToTarget" "SnapToTarget" "KeepRelative" true)
  (CallFunction|BindAmmo)
  (return (.WeaponType (Utilities|Struct|BreakST_WeaponData (Variables|Default|GetWeaponData)))))

(fn EventReload
  (Animation|PlayAnimMontage (Variables|Default|GetCharacter) (.ReloadMontage (Utilities|Struct|BreakST_WeaponData (Variables|Default|GetWeaponData))) 1.0 "None")
  (return false))

(fn EventReloadFinish
  (Utilities|IsOwner?
    (:True
      (if (CallFunction|IsCanChangeMag)
        (CallFunction|ChangeMag)
        (CallFunction|ReqReload)
        (return true)))))

(fn EventTrigger
  (params (IsPressed :type Boolean))
  (if IsPressed
    (bind _iscanfire (CallFunction|IsCanFire))
    (if _iscanfire
      (bind _character (Variables|Default|GetCharacter)
        (:then
          (Animation|PlayAnimMontage _character (.FireMontage (Utilities|Struct|BreakST_WeaponData (Variables|Default|GetWeaponData))) 1.0 "None")
          (return true))
        (:else)))))

(fn IsCanFire
  (return (> (Variables|Default|GetAmmo) 0)))

(fn IsCanReload
  (return (and (< (Variables|Default|GetAmmo) (.MaxAmmo (Utilities|Struct|BreakST_WeaponData (Variables|Default|GetWeaponData)))) (!= (.ReloadMontage (Utilities|Struct|BreakST_WeaponData (Variables|Default|GetWeaponData))) (Animation|Montage|GetCurrentActiveMontage (Components|SkeletalMesh|GetAnimInstance (Variables|/Script/Engine.Character|GetMesh (Variables|Default|GetCharacter))))))))

(fn IsFullAmmo
  (return (>= (Variables|Default|GetAmmo) (.MaxAmmo (Utilities|Struct|BreakST_WeaponData (Variables|Default|GetWeaponData))))))