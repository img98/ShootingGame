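; HUD for the shooting game mode that shows the player's HP, magazine and Sh values.
; On BeginPlay it creates the HUD widget, sets game-only input and hides the cursor.
; It binds to the owning pawn's BP_ShootingPlayerState dispatchers, retrying by timer while the cast fails, and pushes initial values.
; Handler functions forward values to the widget; the ammo handler is not bound here.
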(event EventBeginPlay
  (bind _returnvalue (Game|GetPlayerController 0))
  (Development|PrintString "ShootingHud BeginPlay")
  (bind _returnvalue_2 (UserInterface|CreateWidget "/Game/Shooting/Widget/WBP_ShootingHudWidget.WBP_ShootingHudWidget_C"))
  (bind _output_get (Variables|Default|SetHudWidget _returnvalue_2))
  (UserInterface|Viewport|AddtoViewport _output_get 0)
  (CallFunction|BindMyPlayerState)
  (Input|SetInputModeGameOnly _returnvalue false)
  (Variables|/Script/Engine.PlayerController|SetbShowMouseCursor _returnvalue false))

(fn ConstructionScript)

(fn EventMyUpdateHP
  (params (CurHP :type Float%20%28double-precision%29) (MaxHP :type Float%20%28double-precision%29))
  (Default|UpdateHp (Variables|Default|GetHudWidget) CurHP MaxHP))

(fn BindMyPlayerState
  (bind _asbp_shooting_player_state (Utilities|Casting|CastToBP_ShootingPlayerState (Variables|/Script/Engine.Controller|GetPlayerState (Pawn|GetController (Class|HUD|GetOwningPawn))))
    (:then
      (LocalVariables|SetPlayerState _asbp_shooting_player_state)
      (Utilities|FlowControl|Sequence
        (:then_0
          (CallFunction|EventMyUpdateHP (Variables|/Game/Shooting/GameMode/BP_ShootingPlayerState.BP_ShootingPlayerState_C|GetCurHp (LocalVariables|GetPlayerState)) (Variables|/Game/Shooting/GameMode/BP_ShootingPlayerState.BP_ShootingPlayerState_C|GetMaxHp (LocalVariables|GetPlayerState)))
          (EventDispatchers|BindEventtoEventDispatcherUpdateHP (LocalVariables|GetPlayerState) (EventDispatchers|CreateEvent :!event EventMyUpdateHP)))
        (:then_1
          (CallFunction|EventMyUpdateMag (Variables|/Game/Shooting/GameMode/BP_ShootingPlayerState.BP_ShootingPlayerState_C|GetMag (LocalVariables|GetPlayerState)))
          (EventDispatchers|BindEventtoEventDispatcherUpdateMag (LocalVariables|GetPlayerState) (EventDispatchers|CreateEvent :!event EventMyUpdateMag)))
        (:then_2
          (CallFunction|EventMyUpdateSh (Variables|/Game/Shooting/GameMode/BP_ShootingPlayerState.BP_ShootingPlayerState_C|GetCurSh (LocalVariables|GetPlayerState)) (Variables|/Game/Shooting/GameMode/BP_ShootingPlayerState.BP_ShootingPlayerState_C|GetMaxSh (LocalVariables|GetPlayerState)))
          (EventDispatchers|BindEventtoEventDispatcherUpdateSh (LocalVariables|GetPlayerState) (EventDispatchers|CreateEvent :!event EventMyUpdateSh)))))
    (:CastFailed
      (Utilities|Time|SetTimerbyFunctionName 0 "BindMyPlayerState" 0.01))))

(fn EventMyAmmo
  (params (Ammo :type Integer))
  (Default|UpdateAmmo (Variables|Default|GetHudWidget) Ammo))

(fn EventMyUpdateMag
  (params (Mag :type Integer))
  (Default|UpdateMag (Variables|Default|GetHudWidget) Mag))

(fn EventMyUpdateSh
  (params (CurSh :type Float%20%28double-precision%29) (MaxSh :type Float%20%28double-precision%29))
  (Default|UpdateSh (Variables|Default|GetHudWidget) CurSh MaxSh))